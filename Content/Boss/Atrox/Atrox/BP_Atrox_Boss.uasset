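; Boss character Blueprint for Atrox, driven by an AI controller and Blackboard.
; On BeginPlay it briefly waits, then writes the Player-tagged actor and its location to Blackboard keys.
; SetState mirrors state changes to the Blackboard unless Dead, playing an attack montage on Attack.
; Helper events spawn a scaled attack mesh ahead of an arrow and smoothly yaw the boss toward the stored target location.
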(event Custom|SetState
  (params (NewState :type EBossState%20Enum :default "NewEnumerator0"))
  (if (Utilities|Enum|NotEqual(Enum) (Variables|Default|GetState_BP) "NewEnumerator4")
    (if (Utilities|Enum|NotEqual(Enum) (Variables|Default|GetState_BP) NewState)
      (AI|Components|Blackboard|SetValueasEnum (Variables|/Script/AIModule.AIController|GetBlackboard (AI|GetAIController self)) (Variables|Default|GetStateKey) NewState)
      (bind _output_get (Variables|Default|SetState_BP NewState))
      (switch Utilities|FlowControl|Switch|SwitchonEBossState _output_get
        (:NewEnumerator2
          (Animation|PlayAnimMontage "/Game/Boss/Atrox/Atrox/M_Attack1.M_Attack1" 1.0 "AttackDelay"))))))

(event Custom|SpawnAttackMesh
  (Variables|Default|Setdistance 2e+03)
  (Game|SpawnActorfromClass "/Game/Boss/Atrox/Atrox/BP_Attack1Mesh.BP_Attack1Mesh_C" (Math|Transform|MakeTransform (- (+ (Transformation|GetWorldLocation (Variables|Default|GetArrow1)) (* (Math|Vector|GetForwardVector (Variables|Default|GetArrow1)) (Variables|Default|Getdistance))) "0.000000,0.000000,810.000000") (Transformation|GetWorldRotation (Variables|Default|GetArrow1)) "30.000000,10.000000,1.000000") "Undefined" "MultiplyWithRoot" 0 0))

(event Custom|TurnToTarget
  (bind _returnvalue (Transformation|GetActorLocation))
  (bind _self self)
  (bind _targetplayerlocationkey (Variables|Default|GetTargetPlayerLocationKey))
  (bind _returnvalue_2 (AI|GetAIController _self))
  (bind _returnvalue_3 (AI|GetBlackboard _returnvalue_2))
  (bind _returnvalue_4 (AI|Components|Blackboard|GetValueasVector _returnvalue_3 _targetplayerlocationkey))
  (bind _returnvalue_5 (- _returnvalue_4 _returnvalue))
  (Transformation|SetActorRotation (Math|Interpolation|RInterpTo (Transformation|GetActorRotation) (Math|Rotator|MakeRotfromX (Math|Vector|MakeVector (.x _returnvalue_5) (.y _returnvalue_5) 0.0)) (Utilities|Time|GetWorldDeltaSeconds) 6.0)))

(event EventBeginPlay
  (Utilities|FlowControl|Delay 0.1)
  (bind _outactors (Actor|GetAllActorswithTag "Player"))
  (AI|Components|Blackboard|SetValueasObject (AI|GetBlackboard (AI|GetAIController self)) (Variables|Default|GetTargetPlayerKey) (Utilities|Array|Get(acopy) _outactors))
  (AI|Components|Blackboard|SetValueasVector (AI|GetBlackboard (AI|GetAIController self)) (Variables|Default|GetTargetPlayerLocationKey) (Transformation|GetActorLocation (Utilities|Array|Get(acopy) _outactors))))

(fn ConstructionScript)