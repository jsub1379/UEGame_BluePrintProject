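; BP_Arrow is a flaming arrow projectile that damages actors tagged Boss.
; InitArrow sets its owner, short lifespan, facing and ProjectileMovement speed, and attaches a flamethrower Niagara trail.
; On box overlap with a boss, it applies damage through the instigator, spawns a small explosion facing against its velocity, and destroys itself; other overlaps are ignored.
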(event OnComponentBeginOverlap(BoxCollision)
  (params (OverlappedComponent :type Primitive%20Component%20Object%20Reference) (OtherActor :type Actor%20Object%20Reference) (OtherComp :type Primitive%20Component%20Object%20Reference) (OtherBodyIndex :type Integer) (bFromSweep :type Boolean) (SweepResult :type Hit%20Result%20Structure%20%28by%20ref%29))
  (Utilities|IsValid OtherActor
    (:Is%20Valid
      (if (Actor|ActorHasTag OtherActor "Boss")
        (Game|Damage|ApplyDamage OtherActor (Variables|Default|GetDamage) (Game|GetInstigatorController) self)
        (Niagara|SpawnSystematLocation "/Game/MixedVFX/Particles/Explosions/NS_ExplosionGroundSmall.NS_ExplosionGroundSmall" (Transformation|GetWorldLocation (Variables|Default|GetBoxCollision)) (Math|Conversions|RotationFromXVector (* (Math|Vector|Normalize (Transformation|GetVelocity)) -1.0)))
        (Actor|DestroyActor)))))

(event Custom|InitArrow
  (params (Direction :type Vector) (InSpeed :type Float%20%28double-precision%29) (InOwner :type Actor%20Object%20Reference))
  (Actor|SetOwner InOwner)
  (Actor|SetLifeSpan 3.0)
  (Transformation|SetActorRotation (Math|Rotator|MakeRotfromX Direction))
  (Game|Components|ProjectileMovement|SetVelocityinLocalSpace (Variables|Default|GetProjectileMovement) (Math|Vector|MakeVector InSpeed 0.0 0.0))
  (Variables|Default|SetStartLocation (Transformation|GetActorLocation))
  (Niagara|SpawnSystemAttached "/Game/MixedVFX/Particles/Fires/NS_FlameThrower.NS_FlameThrower" (Variables|Default|GetArrow) "None" "0, 0, 0" "0, 0, 0" "KeepRelativeOffset" true))

(fn ConstructionScript)