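; Damage receiver component that tracks health power and reports changes and death through event dispatchers.
; BeginPlay fills health to the maximum, and OnDamageReceived subtracts incoming damage from it.
; Every hit broadcasts current and maximum health, preceded by OnDead when health is at or below zero.
; Health is not clamped and death is not latched, so further hits broadcast OnDead again while health stays depleted.
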(event Custom|OnDamageReceived
  (params (Damage :type Float%20%28double-precision%29))
  (Variables|Default|SetHealthPower (- (Variables|Default|GetHealthPower) Damage))
  (if (<= (Variables|Default|GetHealthPower) 0.0)
    (Default|CallOnDead)
    (Default|CallOnHealthPoawerChanged (Variables|Default|GetHealthPower) (Variables|Default|GetMaxHealthPower))
    (else
      (Default|CallOnHealthPoawerChanged (Variables|Default|GetHealthPower) (Variables|Default|GetMaxHealthPower)))))

(event EventBeginPlay
  (Variables|Default|SetHealthPower (Variables|Default|GetMaxHealthPower)))